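; BP_PlayerAI is an AI controller that drives a BP_TopDownCharacter through a behavior tree.
; After a short delay on BeginPlay, it caches its controlled pawn and binds TakeOver to that character's GetAI dispatcher.
; TakeOver re-possesses the cached pawn and repeats the binding, letting the AI reclaim the character.
; On possession it prints the player character's name for debugging, stores the pawn and starts the tree after a brief delay.
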(event `self.ReceiveBeginPlay`
  (`KismetSystemLibrary.Delay` 0.2)
  (bind _output_get (set `self.Possessed Pawn` (`self.K2_GetPawn`) :!label _label))
  (bind _asbp_top_down_character (cast `/Game/TopDown/Blueprints/BP_TopDownCharacter` _output_get))
  (add `/Game/TopDown/Blueprints/BP_TopDownCharacter.GetAI` _asbp_top_down_character (delegate `TakeOver`)))

(event `TakeOver`
  (`self.Possess` (`self.Possessed Pawn`))
  (goto _label))

(event `self.ReceivePossess`
  (params (PossessedPawn :type "Pawn Object Reference"))
  (`KismetSystemLibrary.PrintString` (`KismetSystemLibrary.GetDisplayName` (`GameplayStatics.GetPlayerCharacter` 0)))
  (set `self.Possessed Pawn` PossessedPawn)
  (`KismetSystemLibrary.Delay` 0.2)
  (`self.RunBehaviorTree` (`self.BT`)))

(fn `UserConstructionScript`)