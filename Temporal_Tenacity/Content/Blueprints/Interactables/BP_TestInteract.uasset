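; BP_TestInteract is a test interactable actor that gives visual debug feedback when interacted with.
; Its Interact function checks whether the passed reference is itself, then draws a short-lived red debug arrow from the actor to the player character and returns true.
; Any other reference returns false, and the event graph holds only disabled default events.
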(fn `Interact`
  (params (Ref :type "Object Object Reference"))
  (returns (Succ :type Boolean))
  (if (== Ref self)
    (`KismetSystemLibrary.DrawDebugArrow` (`self.K2_GetActorLocation`) (`self.K2_GetActorLocation` (`GameplayStatics.GetPlayerCharacter` 0)) 5.0 (struct :`R` 1.0 :`B` 0.06667 :`A` 1.0) 5.0 2.0)
    (return true)
    (else
      (return false))))

(fn `UserConstructionScript`
  (`parent.UserConstructionScript`))